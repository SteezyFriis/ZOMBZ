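; BP_GeneratorStart is a key-system Blueprint that announces a generator start once both gasoline and gear conditions are met.
; Every Tick it loops over all TannHjul and Gasolina actors with empty bodies, then checks GasAdded and TannHjulEnabled on the last element of each.
; When both are true it prints a message and plays a click sound, repeating each frame because nothing latches the state.
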(event EventTick
  (params (DeltaSeconds :type Float%20%28single-precision%29))
  (Utilities|FlowControl|Sequence
    (:then_0
      (bind _outactors (Actor|GetAllActorsOfClass "/Game/GAME/Blueprints/Key_System/TannHjul.TannHjul_C"))
      (bind _array_element (Utilities|Array|ForEachLoopwithBreak _outactors)))
    (:then_1
      (bind _outactors_2 (Actor|GetAllActorsOfClass "/Game/GAME/Blueprints/Key_System/Gasolina.Gasolina_C"))
      (bind _array_element_2 (Utilities|Array|ForEachLoopwithBreak _outactors_2)))
    (:then_2
      (if (Variables|/Game/GAME/Blueprints/Key_System/Gasolina.Gasolina_C|GetGas_Added _array_element_2)
        (if (Variables|/Game/GAME/Blueprints/Key_System/TannHjul.TannHjul_C|GetTannHjul_enabled _array_element)
          (Development|PrintString "Generator started! " true true "(R=0.000000,G=0.666354,B=1.000000,A=1.000000)")
          (Audio|PlaySound2D "/Game/GAME/Blueprints/MainMenu/MenuAssets/220180__gameaudio__click-pop.220180__gameaudio__click-pop"))))))

(fn ConstructionScript)