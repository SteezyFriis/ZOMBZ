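; BP_BackDoor2 is an interactive back door that the player opens and closes with E, with no key check in this Blueprint.
; An overlap volume enables input while the ThirdPersonCharacter is inside and prints a prompt on screen.
; E plays or reverses a timeline that drives the mesh's relative yaw.
; Tick sets IsClosed whenever that timeline value is below 1, deciding which direction E triggers.
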(event OnComponentBeginOverlap(Overlap)
  (params (OverlappedComponent :type Primitive%20Component%20Object%20Reference) (OtherActor :type Actor%20Object%20Reference) (OtherComp :type Primitive%20Component%20Object%20Reference) (OtherBodyIndex :type Integer) (bFromSweep :type Boolean) (SweepResult :type Hit%20Result%20Structure%20%28by%20ref%29))
  (Utilities|Casting|CastToThirdPersonCharacter OtherActor)
  (Input|EnableInput (Game|GetPlayerController 0))
  (Development|PrintString "PRESS E TO OPEN" true true "(R=0.012200,G=1.000000,B=0.000000,A=1.000000)" 3.0))

(event OnComponentEndOverlap(Overlap)
  (params (OverlappedComponent :type Primitive%20Component%20Object%20Reference) (OtherActor :type Actor%20Object%20Reference) (OtherComp :type Primitive%20Component%20Object%20Reference) (OtherBodyIndex :type Integer))
  (Utilities|Casting|CastToThirdPersonCharacter OtherActor)
  (Input|DisableInput (Game|GetPlayerController 0)))

(event EventTick
  (params (DeltaSeconds :type Float%20%28single-precision%29))
  (Variables|Default|SetIsClosed (< (stale Input|KeyboardEvents|E _backdoor_rot_2) 1.0)))

(event Input|KeyboardEvents|E
  (params (Key :type Key%20Structure))
  (:Pressed
    (if (Variables|Default|GetIsClosed)
      (bind _backdoor_rot_2 (Timeline|Backdoor_rot_2 Play)
        (:Update
          (Transformation|SetRelativeRotation (Variables|Default|GetStaticMesh) (Math|Rotator|MakeRotator 0.0 0.0 _backdoor_rot_2) false false)))
      (else
        (Timeline|Backdoor_rot_2 Reverse)))))

(fn ConstructionScript)