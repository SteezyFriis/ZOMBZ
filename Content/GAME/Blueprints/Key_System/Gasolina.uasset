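; Gasolina is an interactable gas fill point, apparently for a generator, that consumes a required key item from the player.
; Overlapping it enables input and prompts for E, and leaving disables input.
; E searches the character's OwnedKeys for RequireKeyType, removes it and sets GasAdded, though an outer check reads the loop element before the loop runs.
; An unconnected branch would copy OwnedKeys to TestGameInstance but never runs.
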(event OnComponentBeginOverlap(Overlap)
  (params (OverlappedComponent :type Primitive%20Component%20Object%20Reference) (OtherActor :type Actor%20Object%20Reference) (OtherComp :type Primitive%20Component%20Object%20Reference) (OtherBodyIndex :type Integer) (bFromSweep :type Boolean) (SweepResult :type Hit%20Result%20Structure%20%28by%20ref%29))
  (bind _asthird_person_character (Utilities|Casting|CastToThirdPersonCharacter OtherActor))
  (Input|EnableInput (Game|GetPlayerController 0))
  (Development|PrintString "PRESS E TO FILL GAS" true true "(R=0.012200,G=1.000000,B=0.000000,A=1.000000)" 3.0))

(event OnComponentEndOverlap(Overlap)
  (params (OverlappedComponent :type Primitive%20Component%20Object%20Reference) (OtherActor :type Actor%20Object%20Reference) (OtherComp :type Primitive%20Component%20Object%20Reference) (OtherBodyIndex :type Integer))
  (Utilities|Casting|CastToThirdPersonCharacter OtherActor)
  (Input|DisableInput (Game|GetPlayerController 0)))

(event Input|KeyboardEvents|E
  (params (Key :type Key%20Structure))
  (:Pressed
    (if (Utilities|Enum|Equal(Enum) (stale _array_element) (Variables|Default|GetRequire%20Key%20Type))
      (for (_array_element _array_index) (Variables|/Game/GAME/Character/ThirdPersonCharacter.ThirdPersonCharacter_C|GetOwnedKeys (stale OnComponentBeginOverlap(Overlap) _asthird_person_character))
        (if (Utilities|Enum|Equal(Enum) _array_element (Variables|Default|GetRequire%20Key%20Type))
          (Utilities|Array|RemoveIndex (Variables|/Game/GAME/Character/ThirdPersonCharacter.ThirdPersonCharacter_C|GetOwnedKeys (stale OnComponentBeginOverlap(Overlap) _asthird_person_character)) _array_index)
          (Development|PrintString "Generator part added!" true true "(R=0.012200,G=1.000000,B=0.000000,A=1.000000)")
          (if true
            (Variables|Default|SetGas_Added true))))
      (else
        (Development|PrintString "Need Gas" true true "(R=1.000000,G=0.000000,B=0.016751,A=1.000000)" 3.0)))))

(fn ConstructionScript)