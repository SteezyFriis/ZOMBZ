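; Sliding door actor for the Skytower lobby that opens when the player character approaches.
; BeginPlay stores the starting location, and entering the Overlap volume plays a timeline that moves the whole actor by an animated offset from that position.
; When the character leaves the volume, the timeline reverses after a short delay to slide the door back.
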(event OnComponentBeginOverlap(Overlap)
  (params (OverlappedComponent :type Primitive%20Component%20Object%20Reference) (OtherActor :type Actor%20Object%20Reference) (OtherComp :type Primitive%20Component%20Object%20Reference) (OtherBodyIndex :type Integer) (bFromSweep :type Boolean) (SweepResult :type Hit%20Result%20Structure%20%28by%20ref%29))
  (Utilities|Casting|CastToThirdPersonCharacter OtherActor)
  (bind _slidingdoor (Timeline|SlidingDoor1 Play)
    (:Update
      (Transformation|SetActorLocation (+ _slidingdoor (Variables|Default|GetStartingPosition)) false false))))

(event OnComponentEndOverlap(Overlap)
  (params (OverlappedComponent :type Primitive%20Component%20Object%20Reference) (OtherActor :type Actor%20Object%20Reference) (OtherComp :type Primitive%20Component%20Object%20Reference) (OtherBodyIndex :type Integer))
  (Utilities|Casting|CastToThirdPersonCharacter OtherActor)
  (Utilities|FlowControl|Delay 1.0)
  (bind _slidingdoor (Timeline|SlidingDoor1 Reverse)
    (:Update
      (Transformation|SetActorLocation (+ _slidingdoor (Variables|Default|GetStartingPosition)) false false))))

(event EventBeginPlay
  (Variables|Default|SetStartingPosition (Transformation|GetActorLocation)))

(fn ConstructionScript)