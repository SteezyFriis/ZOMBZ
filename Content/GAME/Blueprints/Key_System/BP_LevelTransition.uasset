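; BP_LevelTransition is a key-gated level exit that opens a named level when the third-person character overlaps it with the required key type.
; On overlap it searches the character's OwnedKeys, removes the matching key and opens the level, or otherwise prints "Need key".
; The outer key check reads the loop's element before the loop runs.
; Code copying keys to TestGameInstance is unconnected, so this Blueprint never saves them.
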(event OnComponentBeginOverlap(Overlap)
  (params (OverlappedComponent :type Primitive%20Component%20Object%20Reference) (OtherActor :type Actor%20Object%20Reference) (OtherComp :type Primitive%20Component%20Object%20Reference) (OtherBodyIndex :type Integer) (bFromSweep :type Boolean) (SweepResult :type Hit%20Result%20Structure%20%28by%20ref%29))
  (bind _asthird_person_character (Utilities|Casting|CastToThirdPersonCharacter OtherActor))
  (if (Utilities|Enum|Equal(Enum) (stale _array_element) (Variables|Default|GetRequiredKeyType))
    (for (_array_element _array_index) (Variables|/Game/GAME/Character/ThirdPersonCharacter.ThirdPersonCharacter_C|GetOwnedKeys _asthird_person_character)
      (if (Utilities|Enum|Equal(Enum) _array_element (Variables|Default|GetRequiredKeyType))
        (Utilities|Array|RemoveIndex (Variables|/Game/GAME/Character/ThirdPersonCharacter.ThirdPersonCharacter_C|GetOwnedKeys _asthird_person_character) _array_index)
        (Development|PrintString "")
        (Game|OpenLevel(byName) (Variables|Default|GetLevelName))))
    (else
      (Development|PrintString "Need  key" true true "(R=1.000000,G=0.000000,B=0.016751,A=1.000000)" 5.0))))

(fn ConstructionScript)