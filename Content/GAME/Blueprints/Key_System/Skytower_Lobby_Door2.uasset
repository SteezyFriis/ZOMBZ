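; Sliding door actor for the Skytower lobby that opens automatically when a ThirdPersonCharacter enters its Overlap volume.
; It records its starting location at BeginPlay, then plays the SlidingDoor2 timeline, moving the whole actor by the track offset from that position.
; When the character leaves the volume, it waits one second and reverses the timeline to close.
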(event OnComponentBeginOverlap(Overlap)
  (params (OverlappedComponent :type Primitive%20Component%20Object%20Reference) (OtherActor :type Actor%20Object%20Reference) (OtherComp :type Primitive%20Component%20Object%20Reference) (OtherBodyIndex :type Integer) (bFromSweep :type Boolean) (SweepResult :type Hit%20Result%20Structure%20%28by%20ref%29))
  (Utilities|Casting|CastToThirdPersonCharacter OtherActor)
  (bind _newtrack_0 (Timeline|SlidingDoor2 Play)
    (:Update
      (Transformation|SetActorLocation (+ _newtrack_0 (Variables|Default|GetStartingPosition)) false false))))

(event OnComponentEndOverlap(Overlap)
  (params (OverlappedComponent :type Primitive%20Component%20Object%20Reference) (OtherActor :type Actor%20Object%20Reference) (OtherComp :type Primitive%20Component%20Object%20Reference) (OtherBodyIndex :type Integer))
  (Utilities|Casting|CastToThirdPersonCharacter OtherActor)
  (Utilities|FlowControl|Delay 1.0)
  (bind _newtrack_0 (Timeline|SlidingDoor2 Reverse)
    (:Update
      (Transformation|SetActorLocation (+ _newtrack_0 (Variables|Default|GetStartingPosition)) false false))))

(event EventBeginPlay
  (Variables|Default|SetStartingPosition (Transformation|GetActorLocation)))

(fn ConstructionScript)