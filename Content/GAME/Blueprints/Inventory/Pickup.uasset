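; Pickup actor that adds an item to the player's inventory when the ThirdPersonCharacter touches it.
; The construction script picks the static mesh from a Meshes array by Index.
; Overlap on either the Overlap component or the mesh finds the first top-level Inventory widget, passes it the same Index via Additem, then destroys the actor.
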(event OnComponentBeginOverlap(Overlap)
  (params (OverlappedComponent :type Primitive%20Component%20Object%20Reference) (OtherActor :type Actor%20Object%20Reference) (OtherComp :type Primitive%20Component%20Object%20Reference) (OtherBodyIndex :type Integer) (bFromSweep :type Boolean) (SweepResult :type Hit%20Result%20Structure%20%28by%20ref%29))
  (Utilities|Casting|CastToThirdPersonCharacter OtherActor)
  (bind _foundwidgets (Widget|GetAllWidgetsOfClass "/Game/GAME/Blueprints/Inventory/Inventory.Inventory_C" true))
  (Default|Additem (Utilities|Array|Get(acopy) _foundwidgets) (Variables|Default|Getindex))
  (Actor|DestroyActor))

(event OnComponentBeginOverlap(StaticMesh)
  (params (OverlappedComponent :type Primitive%20Component%20Object%20Reference) (OtherActor :type Actor%20Object%20Reference) (OtherComp :type Primitive%20Component%20Object%20Reference) (OtherBodyIndex :type Integer) (bFromSweep :type Boolean) (SweepResult :type Hit%20Result%20Structure%20%28by%20ref%29))
  (Utilities|Casting|CastToThirdPersonCharacter (stale OnComponentBeginOverlap(Overlap) OtherActor))
  (bind _foundwidgets (Widget|GetAllWidgetsOfClass "/Game/GAME/Blueprints/Inventory/Inventory.Inventory_C" true))
  (Default|Additem (Utilities|Array|Get(acopy) _foundwidgets) (Variables|Default|Getindex))
  (Actor|DestroyActor))

(event EventBeginPlay)

(event Collision|EventActorBeginOverlap
  (params (OtherActor :type Actor%20Object%20Reference)))

(event EventTick
  (params (DeltaSeconds :type Float%20%28single-precision%29)))

(fn ConstructionScript
  (Components|StaticMesh|SetStaticMesh (Variables|Default|GetStaticMesh) (Utilities|Array|Get(acopy) (Variables|Default|GetMeshes) (Variables|Default|Getindex))))